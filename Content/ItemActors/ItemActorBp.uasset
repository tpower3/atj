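; Item actor that displays its item name as floating text in the world.
; The construction script passes ItemName to SetName, writes it to the TextRender and gives the text a random RGB color.
; Tick rotates the text each frame to face the player camera manager.
; A GetName override returns ItemName without calling the parent version.
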(event EventBeginPlay)

(event Collision|EventActorBeginOverlap
  (params (OtherActor :type Actor%20Object%20Reference)))

(event EventTick
  (params (DeltaSeconds :type Float%20%28single-precision%29))
  (bind _textrender (Variables|Default|GetTextRender))
  ;[1 1 1] Rotate Text to Face Camera
  (Transformation|SetWorldRotation _textrender (Math|Rotator|FindLookatRotation (Transformation|GetWorldLocation _textrender) (Transformation|GetActorLocation (Game|GetPlayerCameraManager 0))) false false))

(fn ConstructionScript
  (bind _itemname (Variables|Default|GetitemName))
  (bind _textrender (Variables|Default|GetTextRender))
  (Class|ItemActor|SetName _itemname)
  (Rendering|Components|TextRender|SetText _textrender (Utilities|Text|ToText(String) _itemname))
  (Rendering|Components|TextRender|SetTextRenderColor _textrender (Math|Color|MakeColor (Math|Conversions|ToByte(Integer) (Class|KismetMathLibrary|RandomInteger64inRange 0 255)) (Math|Conversions|ToByte(Integer) (Class|KismetMathLibrary|RandomInteger64inRange 0 255)) (Math|Conversions|ToByte(Integer) (Class|KismetMathLibrary|RandomInteger64inRange 0 255)))))

(fn GetName
  (return (Variables|Default|GetitemName)))